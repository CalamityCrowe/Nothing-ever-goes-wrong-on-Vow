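; BP_Turret is a hazard turret Blueprint that tracks a spin with wind-up and wind-down.
; BeginPlay plays the TurretWindUp timeline, whose Alpha sets SpinSpeed, and StopTurretRotation reverses it to wind down.
; Tick accumulates SpinSpeed scaled by delta time into CurrentSpinRot.
; The graph never applies that value to TurretMesh, which is unreferenced.
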(event `Begin Turret Rotation`
  (bind (_direction _alpha) (`Timeline|Turret Wind-Up` :!label _label)
    (:`Update`
      (set `self.SpinSpeed` _alpha))))

(event `Stop Turret Rotation`
  (goto _label :!via `Reverse`))

(event `self.ReceiveBeginPlay`
  (`self.Begin Turret Rotation`))

(event `self.ReceiveTick`
  (params (DeltaSeconds :type "Float (single-precision)"))
  (set `self.CurrentSpinRot` (+ (`self.CurrentSpinRot`) (* DeltaSeconds (`self.SpinSpeed`)))))

(fn `UserConstructionScript`)