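; Procedural dungeon generator actor that builds a layout of connected rooms on BeginPlay.
; It spawns a start room at its root transform and pools the child components of that room's ExitsFolder as open exits.
; It then recursively spawns random RoomList classes at random exits, adding each Master_Room's exits and removing the used one until RoomAmount runs out.
; Rooms always spawn, with no overlap check.
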(event `Spawn Start Room`
  (bind _exits (`self.Exits`))
  ;[0 1 0.1073] Spawn Start Room
  (bind _returnvalue (`|SpawnActorFromClass` "/Game/Blueprints/Procedural/Dungeon_Room1.Dungeon_Room1_C" (`SceneComponent.K2_GetComponentToWorld` (`self.DefaultSceneRoot`)) "AlwaysSpawn" "MultiplyWithRoot" null null))
  (`KismetArrayLibrary.Array_Append` _exits (`SceneComponent.GetChildrenComponents` (`/Game/Blueprints/Procedural/Master_Room.ExitsFolder` _returnvalue) false))
  (`KismetSystemLibrary.PrintString` (`KismetStringLibrary.Conv_IntToString` (`KismetArrayLibrary.Array_Length` _exits))))

(event `Spawn Next room`
  ;[0 1 0.2847] Spawn New Room
  (bind _output_get (set `self.Selected Exit Point` (`KismetArrayLibrary.Array_Random` (`self.Exits`))))
  (bind _returnvalue (`|SpawnActorFromClass` (`KismetArrayLibrary.Array_Random` (`self.Room List`)) (`SceneComponent.K2_GetComponentToWorld` _output_get) "AlwaysSpawn" "MultiplyWithRoot" null null))
  (bind _asmaster_room (cast `/Game/Blueprints/Procedural/Master_Room` _returnvalue))
  (bind _output_get_2 (set `self.Latest Room` _asmaster_room))
  (`KismetArrayLibrary.Array_Append` (`self.Exits`) (`SceneComponent.GetChildrenComponents` (`/Game/Blueprints/Procedural/Master_Room.ExitsFolder` _output_get_2) false))
  (`KismetArrayLibrary.Array_RemoveItem` (`self.Exits`) (`self.Selected Exit Point`))
  (bind _result (`/Engine/EditorBlueprintResources/StandardMacros.DecrementInt` (`self.Room Amount`))
    (:`  `
      (if (> _result 0)
        (`self.Spawn Next room`)))))

(event `self.ReceiveBeginPlay`
  (`self.Spawn Start Room `)
  (`self.Spawn Next room`))

(fn `UserConstructionScript`)